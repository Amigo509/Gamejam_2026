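; BP_Door is an interactable hinged door that swings open and closed.
; Each Interact call toggles the Opening state and plays or reverses a single timeline, which interpolates the Door component's relative yaw between closed and a quarter turn open.
; An IsDoorMoving flag ignores further interactions until the timeline finishes.
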(event `/Game/Interface/BPI_Interaction.Interact`
  (if (not (`self.bIsDoorMoving`))
    (set `self.bIsDoorMoving` true)
    (bind _output_get (set `self.bOpening` (not (`self.bOpening`))))
    (if _output_get
      (bind (_direction _alpha) (`Timeline|DoorTimeLine` :!label _label)
        (:`Update`
          (`SceneComponent.K2_SetRelativeRotation` (`self.Door`) (`KismetMathLibrary.MakeRotator` 0.0 0.0 (`KismetMathLibrary.Lerp` 0.0 -90.0 _alpha)) false false))
        (:`Finished`
          (set `self.bIsDoorMoving` false)))
      (else
        (goto _label :!via `Reverse`)))))

(fn `UserConstructionScript`)