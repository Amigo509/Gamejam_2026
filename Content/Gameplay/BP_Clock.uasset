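; BP_Clock decides and shows the game's end result once its TimeExpired flag is set.
; The Vars event stores four booleans passed in from outside.
; While TimeExpired is true, Tick creates an animated win screen if all four are true, otherwise an animated lose screen.
; No guard stops this repeating, so a new widget is added every frame the flag stays true.
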(event `self.ReceiveTick`
  (params (DeltaSeconds :type "Float (single-precision)"))
  (if (`self.bTimeExpired`)
    (if (and (`self.NewVar`) (`self.NewVar_0`) (`self.NewVar_1`) (`self.NewVar_2`))
      (bind _returnvalue (`|CreateWidget` "/Game/ThirdPerson/Blueprints/WBP_WinScreen.WBP_WinScreen_C"))
      (`UserWidget.AddToViewport` _returnvalue 0)
      (`UserWidget.PlayAnimation` _returnvalue (`/Game/ThirdPerson/Blueprints/WBP_WinScreen.Animation` _returnvalue) 0.0 1 "Forward" 1.0 false)
      (else
        (bind _returnvalue_2 (`|CreateWidget` "/Game/ThirdPerson/Blueprints/WBP_LoseScreen.WBP_LoseScreen_C"))
        (`UserWidget.AddToViewport` _returnvalue_2 0)
        (`UserWidget.PlayAnimation` _returnvalue_2 (`/Game/ThirdPerson/Blueprints/WBP_LoseScreen.Animation` _returnvalue_2) 0.0 1 "Forward" 1.0 false)))))

(event `/Game/Interface/BPI_Var.Vars`
  (params (b1 :type Boolean) (b2 :type Boolean) (b3 :type Boolean) (b4 :type Boolean))
  (set `self.NewVar` b1)
  (set `self.NewVar_0` b2)
  (set `self.NewVar_1` b3)
  (set `self.NewVar_2` b4))

(fn `UserConstructionScript`)